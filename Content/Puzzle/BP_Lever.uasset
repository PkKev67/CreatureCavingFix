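; BP_Lever is a puzzle lever that triggers a set of linked target objects when pushed.
; On BeginPlay it passes its first actor tag to the player character through an interface message and caches the returned target references.
; Each Push uses a FlipFlop to snap the lever mesh between two tilted poses, then sends a Trigger interface message to every target.
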(event EventBeginPlay
  (bind _target_references (Class|BPIStandard|GetObjectTargets(Message) (Game|GetPlayerCharacter 0) (Utilities|Array|Get(acopy) (Variables|Actor|GetTags))))
  (Variables|Default|SetTarget%20References _target_references))

(event EventPush
  (bind _lever (Variables|Default|GetLever))
  (Utilities|FlowControl|FlipFlop
    (:A
      (Transformation|SetRelativeLocationAndRotation _lever "10.000000,0.000000,10.000000" "-35.000000,0.000000,0.000000" false false))
    (:B
      (Transformation|SetRelativeLocationAndRotation _lever "-10.000000,0.000000,10.000000" "35.000000,0.000000,0.000000" false false)))
  (for _array_element (Variables|Default|GetTarget%20References)
    (Class|BPIStandard|Trigger(Message) _array_element)))

(fn ConstructionScript)

(fn GetObjectTargets
  (params (Target_name :type Name :default "None"))
  (return 0))