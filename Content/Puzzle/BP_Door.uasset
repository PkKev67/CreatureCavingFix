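; Puzzle door actor that slides its Door component downward when its Trigger event fires.
; Tick starts disabled; Trigger resets a counter and enables it, then each tick lowers the door a fixed step until the count passes its limit and Tick switches off.
; Movement is frame-based rather than scaled by delta time, and nothing raises the door again.
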(event EventBeginPlay
  (Actor|Tick|SetActorTickEnabled false))

(event EventTick
  (params (DeltaSeconds :type Float%20%28single-precision%29))
  (bind _door (Variables|Default|GetDoor))
  (bind _count (Variables|Default|Getcount))
  (bind _relativelocation (Variables|/Script/Engine.SceneComponent|GetRelativeLocation _door))
  (Transformation|SetRelativeLocation _door (Math|Vector|MakeVector (.x _relativelocation) (.y _relativelocation) (+ (.z _relativelocation) -15.0)) false false)
  (if (> _count 12)
    (Actor|Tick|SetActorTickEnabled false)
    (else
      (Math|Integer|IncrementInt _count))))

(event EventTrigger
  (Actor|Tick|SetActorTickEnabled true)
  (Variables|Default|Setcount 0))

(fn ConstructionScript)

(fn GetObjectTargets
  (params (Target_name :type Name :default "None"))
  (return 0))