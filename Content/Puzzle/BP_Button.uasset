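; Puzzle button that triggers a set of target objects when pushed.
; On BeginPlay it asks the player character for the targets matching its first actor tag and caches them.
; Push snaps the button mesh to the body's position, restarts Tick and sends a trigger message to each target.
; Tick raises the button by a fixed step per frame, then disables itself after a few frames.
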(event EventTick
  (params (DeltaSeconds :type Float%20%28single-precision%29))
  (bind _button (Variables|Default|GetButton))
  (bind _count (Variables|Default|GetCount))
  (bind _relativelocation (Variables|/Script/Engine.SceneComponent|GetRelativeLocation _button))
  (Transformation|SetRelativeLocation _button (Math|Vector|MakeVector (.x _relativelocation) (.y _relativelocation) (+ (.z _relativelocation) 7.0)) false false)
  (if (> _count 5)
    (Actor|Tick|SetActorTickEnabled false)
    (else
      (Math|Integer|IncrementInt _count))))

(event EventPush
  (Transformation|SetRelativeLocation (Variables|Default|GetButton) (Variables|/Script/Engine.SceneComponent|GetRelativeLocation (Variables|Default|GetBody)) false false)
  (Actor|Tick|SetActorTickEnabled true)
  (Variables|Default|SetCount 0)
  (for _array_element (Variables|Default|GetTarget%20References)
    (Class|BPIStandard|Trigger(Message) _array_element)))

(event EventBeginPlay
  (bind _target_references (Class|BPIStandard|GetObjectTargets(Message) (Game|GetPlayerCharacter 0) (Utilities|Array|Get(acopy) (Variables|Actor|GetTags))))
  (Variables|Default|SetTarget%20References _target_references))

(fn ConstructionScript)

(fn GetObjectTargets
  (params (Target_name :type Name :default "None"))
  (return 0))